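; Player character for a survival game that loses health outside light, with world-axis movement, a melee knockback and placeable lights.
; A looping timer checks registered game-state lights by distance and visibility trace, applying damage when none qualifies.
; BasicAttack pushes overlapping enemies along control-rotation forward, then waits out a cooldown.
; Action spawns and registers a light at the player, movement input sets control rotation, and Q opens the main menu.
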(event Custom|DamageIfNotInLight
  ;[1 1 1] Check Lights
  (CallFunction|CalculateinLight)
  (if (Variables|Default|GetinLight)
    _
    (else
      (Class|BaseCharacter|CalculateHealth -1.0)))
  (Development|PrintString (Utilities|String|Append "Health: " (Utilities|String|ToString(Float) (Variables|Default|GetHealth)))))

(event EventBeginPlay
  ;[1 1 1] Begin Play
  (Utilities|FlowControl|Sequence
    (:then_0
      (bind _asue4survival_game_state (Utilities|Casting|CastToUE4SurvivalGameState (Game|GetGameState)))
      (Variables|Default|SetGameStateRef _asue4survival_game_state))
    (:then_1
      (Utilities|Time|SetTimerbyFunctionName 0 "DamageIfNotInLight" 2.0 true))))

(event Input|ActionEvents|InputActionBasicAttack
  (params (Key :type Key%20Structure))
  (bind _attackarea (Variables|Default|GetAttackArea))
  (bind _overlappingactors (Collision|GetOverlappingActors _attackarea "/Game/Blueprints/EnemyCharacter.EnemyCharacter_C" :!class /Script/Engine.PrimitiveComponent))
  ;[1 1 1] BasicAttack
  (:Pressed
    (if (Variables|Default|GetCanAttack)
      (if (>= (Utilities|Array|LastIndex _overlappingactors) 0)
        (CallFunction|SetCanAttack false)
        (for _array_element _overlappingactors
          (bind _asenemy_character (Utilities|Casting|CastToEnemyCharacter _array_element))
          (Class|NavMovementComponent|StopActiveMovement (Variables|/Script/Engine.Character|GetCharacterMovement _asenemy_character))
          (Components|Movement|StopMovementImmediately (Variables|/Script/Engine.Character|GetCharacterMovement _asenemy_character))
          (Physics|AddImpulse (Variables|/Script/Engine.Character|GetCharacterMovement _asenemy_character) (CallFunction|CalculateMeleeForce) false)
          (Development|PrintString "TargetHt"))
        (Utilities|FlowControl|Delay (Variables|Default|GetAttackDelay))
        (CallFunction|SetCanAttack true)))))

(event Input|ActionEvents|InputActionAction
  (params (Key :type Key%20Structure))
  ;[1 1 1] Spawn Light
  (:Pressed
    (bind _returnvalue (Game|SpawnActorfromClass "/Game/Blueprints/LightSource.LightSource_C" (Transformation|GetActorTransform self) "Undefined" 0 0))
    (Default|AddLightSource (Variables|Default|GetGameStateRef) _returnvalue)))

(event Input|AxisEvents|InputAxisMoveUp
  (params (AxisValue :type Float%20%28single-precision%29))
  ;[1 1 1] Movement/Rotation
  (Pawn|Input|AddMovementInput "1.000000, 0, 0" AxisValue false)
  (if (> (Math|Vector|VectorLength (Math|Vector|MakeVector AxisValue (stale Input|AxisEvents|InputAxisMoveRight AxisValue) 0.0)) 0.5)
    (Pawn|SetControlRotation (Pawn|GetController) (Math|Conversions|RotationFromXVector (Math|Vector|MakeVector AxisValue (stale Input|AxisEvents|InputAxisMoveRight AxisValue) 0.0)))))

(event Input|AxisEvents|InputAxisMoveRight
  (params (AxisValue :type Float%20%28single-precision%29))
  ;[1 1 1] Movement/Rotation
  (Pawn|Input|AddMovementInput "0.000000,1.000000, 0" AxisValue false)
  (if (> (Math|Vector|VectorLength (Math|Vector|MakeVector (stale Input|AxisEvents|InputAxisMoveUp AxisValue) AxisValue 0.0)) 0.5)
    (Pawn|SetControlRotation (Pawn|GetController) (Math|Conversions|RotationFromXVector (Math|Vector|MakeVector (stale Input|AxisEvents|InputAxisMoveUp AxisValue) AxisValue 0.0)))))

(event Input|KeyboardEvents|Q
  (params (Key :type Key%20Structure))
  (:Pressed
    (Game|OpenLevel(byName) "MainMenu")))

(fn ConstructionScript)

(fn CalculateMeleeForce
  (return (* (Math|Vector|GetForwardVector (Pawn|GetControlRotation :!class /Script/Engine.Pawn)) (Variables|Default|GetStrength))))

(fn CalculateinLight
  (bind _self self)
  (bind _array_element (Utilities|Array|ForEachLoopwithBreak (Default|GetLightSources (Variables|Default|GetGameStateRef)) :!label _label)
    (:LoopBody
      (if (< (Transformation|GetDistanceTo _self _array_element) 5e+02)
        (bind _returnvalue (Collision|LineTraceByChannel (Transformation|GetActorLocation _self) (Transformation|GetActorLocation _array_element) "TraceTypeQuery1" false 0 "None"))
        (if (not _returnvalue)
          (Variables|Default|SetinLight true)
          (goto _label Break)
          (else
            _)))
      (Variables|Default|SetinLight false))
    (:Completed
      (return))))

(fn SetCanAttack
  (params (CanAttack :type Boolean))
  (Variables|Default|SetCanAttack CanAttack)
  (return))